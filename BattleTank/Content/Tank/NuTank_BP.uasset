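; Player-controllable tank pawn Blueprint that wires input and components for driving, aiming, firing and camera switching.
; On BeginPlay it hands the barrel, turret and tracks to the TankAiming and TankMovement components, and links itself to its HealthBar widget.
; Drive and fire inputs forward to those components, while look axes rotate an azimuth gimbal and spring arm.
; A swap action toggles first- and third-person cameras.
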(event EventBeginPlay
  (Class|TankAimingComponent|Initialise (Variables|Default|GetTankAiming) (Variables|Default|GetBarrel) (Variables|Default|GetTurret))
  (Class|TankMovementComponent|Initialize (Variables|Default|GetTankMovement) (Variables|Default|GetLeft%20Track) (Variables|Default|GetRight%20Track))
  (Components|StaticMesh|SetStaticMesh (Variables|Default|GetBarrel) "/Game/Tank/tank_fbx_Barrel.tank_fbx_Barrel")
  (CallFunction|InitializeHealthBarWidget))

(event Input|ActionEvents|InputActionSwapCamera
  (params (Key :type Key%20Structure :default "None"))
  ;[1 1 1] Camera Swapping
  (:Pressed
    (Components|Activation|ToggleActive (Variables|Default|GetFirstPersonCamera))
    (Components|Activation|ToggleActive (Variables|Default|GetThirdPersonCamera))))

(event Input|ActionEvents|InputActionFire
  (params (Key :type Key%20Structure :default "None"))
  ;[1 1 1] Aiming Input Binding
  (:Pressed
    (Class|TankAimingComponent|Fire (Variables|Default|GetTankAiming))))

(event Input|AxisEvents|InputAxisForward
  (params (AxisValue :type Float%20%28single-precision%29))
  ;[1 1 1] Movement Input Component
  (Class|TankMovementComponent|IntendMoveForward (Variables|Default|GetTankMovement) AxisValue))

(event Input|AxisEvents|InputAxisTurnRight
  (params (AxisValue :type Float%20%28single-precision%29))
  ;[1 1 1] Movement Input Component
  (Development|PrintString (Utilities|String|ToString(Float) AxisValue) true true "(R=0.000000,G=0.660000,B=1.000000,A=1.000000)" AxisValue)
  (Class|TankMovementComponent|IntendTurnRight (Variables|Default|GetTankMovement) AxisValue))

(event Input|AxisEvents|InputAxisAzimuth
  (params (AxisValue :type Float%20%28single-precision%29))
  ;[1 1 1] Aiming Input Binding
  (Transformation|AddLocalRotation (Variables|Default|GetAzimuth%20Gimbal) (Math|Rotator|MakeRotator 0.0 0.0 AxisValue) false false))

(event Input|AxisEvents|InputAxisAzimuthElevation
  (params (AxisValue :type Float%20%28single-precision%29))
  ;[1 1 1] Aiming Input Binding
  (Transformation|AddLocalRotation (Variables|Default|GetSpringArm) (Math|Rotator|MakeRotator 0.0 AxisValue 0.0) false false))

(fn ConstructionScript)

(fn InitializeHealthBarWidget
  (bind _ashealth_bar (Utilities|Casting|CastToHealthBar (UserInterface|GetUserWidgetObject (Variables|Default|GetHealth%20Bar)))
    (:then
      (Variables|/Game/UI/HealthBar.HealthBar_C|SetMyTank _ashealth_bar self))
    (:CastFailed
      _))
  (return))