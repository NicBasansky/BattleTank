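; Mortar actor Blueprint that sets up a mortar's aiming and health display.
; On BeginPlay it initialises the TankAiming component, reusing the tank aiming setup with MortarBarrel as the barrel and Dome as the turret.
; It then casts the HealthBar component's user widget to HealthBar and sets its MyTank reference to itself, linking the widget to this mortar.
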(event EventBeginPlay
  (Class|TankAimingComponent|Initialise (Variables|Default|GetTankAiming) (Variables|Default|GetMortarBarrel) (Variables|Default|GetDome))
  (CallFunction|InitHealthBar))

(fn ConstructionScript)

(fn InitHealthBar
  (bind _ashealth_bar (Utilities|Casting|CastToHealthBar (UserInterface|GetUserWidgetObject (Variables|Default|GetHealth%20Bar)))
    (:then
      (Variables|/Game/UI/HealthBar.HealthBar_C|SetMyTank _ashealth_bar self))
    (:CastFailed
      _))
  (return))